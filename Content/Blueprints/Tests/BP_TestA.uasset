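; BP_TestA is a test actor that exercises Blueprint basics: conditions, text formatting and enums.
; The construction script writes MyName into a TextRender as a name label, and BeginPlay prints a greeting when a numeric or name check passes.
; An unconnected chain would step the TrafficLight enum through its states with delays, showing each on the TextRender, but it never runs.
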(event `self.ReceiveBeginPlay`
  (if (or (>= (`self.NewVar_3`) 0.0) (== (`self.MyName`) "bob"))
    (`KismetSystemLibrary.PrintString` "Hello")))

(event `self.ReceiveTick`
  (params (DeltaSeconds :type "Float (single-precision)")))

(fn `UserConstructionScript`
  (`TextRenderComponent.K2_SetText` (`self.TextRender`) (`|FormatText` "My name is {Name}" (`self.MyName`))))